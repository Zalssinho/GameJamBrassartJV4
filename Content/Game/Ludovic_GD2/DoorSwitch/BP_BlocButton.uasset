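; BP_BlocButton is a one-shot trigger that produces a new pushable block when a BP_BlockPush enters its BoxCollision.
; The overlap plays the BlocSpawn timeline, which raises the NewCube component along Z from its starting relative location.
; When the timeline finishes, a DoOnce hides NewCube, spawns a real BP_BlockPush at its world location with a downward offset, and destroys the button actor.
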(event OnComponentBeginOverlap(BoxCollision)
  (params (OverlappedComponent :type Primitive%20Component%20Object%20Reference) (OtherActor :type Actor%20Object%20Reference) (OtherComp :type Primitive%20Component%20Object%20Reference) (OtherBodyIndex :type Integer) (bFromSweep :type Boolean) (SweepResult :type Hit%20Result%20Structure%20%28by%20ref%29))
  (bind _newcube (Variables|Default|GetNewCube))
  (bind _returnvalue (Transformation|GetWorldLocation _newcube))
  (Utilities|Casting|CastToBP_BlockPush OtherActor)
  (Variables|Default|SetRelativeLocationNewCube (Variables|/Script/Engine.SceneComponent|GetRelativeLocation (Variables|Default|GetNewCube)))
  (bind _newtrack_0 (Timeline|BlocSpawn Play)
    (:Update
      (Transformation|SetRelativeLocation (Variables|Default|GetNewCube) (Math|Vector|MakeVector (.x (Variables|Default|GetRelativeLocationNewCube)) (.y (Variables|Default|GetRelativeLocationNewCube)) (+ (.z (Variables|Default|GetRelativeLocationNewCube)) (Math|Float|Lerp 0.0 275.0 _newtrack_0))) false false))
    (:Finished
      (Utilities|FlowControl|DoOnce false
        (:Completed
          (Rendering|SetVisibility (Variables|Default|GetNewCube) false false)
          (Game|SpawnActorfromClass "/Game/Game/Ludovic_GD2/PushingBlock/BP_BlockPush.BP_BlockPush_C" (Math|Transform|MakeTransform (Math|Vector|MakeVector (.x _returnvalue) (.y _returnvalue) (- (.z _returnvalue) 1.2e+02)) "0, 0, 0" "1.000000,1.000000,1.000000") "Undefined" "MultiplyWithRoot" 0 0)
          (Actor|DestroyActor))))))

(fn ConstructionScript)