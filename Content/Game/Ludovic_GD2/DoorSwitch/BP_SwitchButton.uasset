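; BP_SwitchButton is a pressure switch that activates every linked door in DoorActivate while overlapped and deactivates them when overlap ends.
; A timeline lowers or raises the button meshes by animating relative Z, playing on overlap and reversing on exit.
; When a BP_BlockPush first enters BoxCollision, its cube snaps above the button, MakeCubeOnSwitch is called, and IsTaken prevents further snaps.
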(event OnComponentBeginOverlap(BoxCollision)
  (params (OverlappedComponent :type Primitive%20Component%20Object%20Reference) (OtherActor :type Actor%20Object%20Reference) (OtherComp :type Primitive%20Component%20Object%20Reference) (OtherBodyIndex :type Integer) (bFromSweep :type Boolean) (SweepResult :type Hit%20Result%20Structure%20%28by%20ref%29))
  (bind _button (Variables|Default|GetButton))
  (bind _returnvalue (Transformation|GetWorldLocation _button))
  (bind _asbp_block_push (Utilities|Casting|CastToBP_BlockPush OtherActor))
  (if (not (Variables|Default|GetisTaken))
    (Transformation|SetWorldLocation (Variables|/Game/Game/Ludovic_GD2/PushingBlock/BP_BlockPush.BP_BlockPush_C|GetCube _asbp_block_push) (Math|Vector|MakeVector (.x _returnvalue) (.y _returnvalue) (+ (.z _returnvalue) 8e+01)) false false)
    (Default|MakeCubeonSwitch _asbp_block_push)
    (Variables|Default|SetisTaken true)))

(event Collision|EventActorBeginOverlap
  (params (OtherActor :type Actor%20Object%20Reference))
  ;[1 1 1] Active Door
  (for _array_element (Variables|Default|GetDoorActivate)
    (Default|DoorActive _array_element)
    (bind _switchbutton_ (Timeline|ButtonSwitch Play)
      (:Update
        (Transformation|SetRelativeLocation (Variables|Default|GetButton) (Math|Vector|MakeVector 0.0 0.0 _switchbutton_) false false)))))

(event Collision|EventActorEndOverlap
  (params (OtherActor :type Actor%20Object%20Reference))
  ;[1 1 1] Active Door
  (for _array_element (Variables|Default|GetDoorActivate)
    (Default|DoorDeactivate _array_element)
    (bind _switchbutton_ (Timeline|ButtonSwitch Reverse)
      (:Update
        (Transformation|SetRelativeLocation (Variables|Default|GetButton) (Math|Vector|MakeVector 0.0 0.0 _switchbutton_) false false)))))

(fn ConstructionScript)