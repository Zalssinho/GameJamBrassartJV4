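; BP_Door is a puzzle door that opens once enough linked switches are active.
; DoorActive and DoorDeactivate raise or lower a switch counter and compare it to NumberOfSwitch.
; Meeting the threshold plays the DoorTiming timeline to move the Door and MetalDoor components along Z, while falling short reverses it.
; Both outcomes play the puzzle validation sound at the world origin.
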(event Custom|DoorActive
  ;[1 1 1] SwitchButton and Door Active
  (Math|Integer|IncrementInt (Variables|Default|GetSwitchActivate)
    (:%20%20
      (if (>= (Variables|Default|GetSwitchActivate) (Variables|Default|GetNumberOfSwitch))
        (Audio|PlaySoundatLocation "/Game/Game/SoundDesign/Cue/Validation_du_puzzle_Cue.Validation_du_puzzle_Cue" "0, 0, 0" "0, 0, 0" 1.0 1.0 0.0 0 0 0 0)
        (bind _doortiming (Timeline|DoorTiming Play)
          (:Update
            (Transformation|SetRelativeLocation (Variables|Default|GetDoor) (Math|Vector|MakeVector 0.0 0.0 _doortiming) false false)))
        (else
          (Audio|PlaySoundatLocation "/Game/Game/SoundDesign/Cue/Validation_du_puzzle_Cue.Validation_du_puzzle_Cue" "0, 0, 0" "0, 0, 0" 1.0 1.0 0.0 0 0 0 0)
          (Timeline|DoorTiming Reverse))))))

(event Custom|DoorDeactivate
  ;[1 1 1] SwitchButton and Door Active
  (Math|Integer|DecrementInt (Variables|Default|GetSwitchActivate)
    (:%20%20
      (if (>= (Variables|Default|GetSwitchActivate) (Variables|Default|GetNumberOfSwitch))
        (Audio|PlaySoundatLocation "/Game/Game/SoundDesign/Cue/Validation_du_puzzle_Cue.Validation_du_puzzle_Cue" "0, 0, 0" "0, 0, 0" 1.0 1.0 0.0 0 0 0 0)
        (bind _doortiming (Timeline|DoorTiming Play)
          (:Update
            (Transformation|SetRelativeLocation (Variables|Default|GetDoor) (Math|Vector|MakeVector 0.0 0.0 _doortiming) false false)))
        (else
          (Audio|PlaySoundatLocation "/Game/Game/SoundDesign/Cue/Validation_du_puzzle_Cue.Validation_du_puzzle_Cue" "0, 0, 0" "0, 0, 0" 1.0 1.0 0.0 0 0 0 0)
          (Timeline|DoorTiming Reverse))))))

(fn ConstructionScript)