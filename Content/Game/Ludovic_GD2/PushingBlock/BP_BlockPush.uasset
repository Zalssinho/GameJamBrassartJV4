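; BP_BlockPush is a block the player can propel, which destroys enemies it hits while moving.
; PropulseBlock enables physics and applies a velocity-change impulse along X or Y only, whichever first exceeds a threshold, with X checked first.
; Box overlaps stop the block shortly after touching walls and toggle a player HUD prompt.
; MakeCubeOnSwitch locks the block by disabling propulsion and physics.
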(event OnComponentEndOverlap(Box)
  (params (OverlappedComponent :type Primitive%20Component%20Object%20Reference) (OtherActor :type Actor%20Object%20Reference) (OtherComp :type Primitive%20Component%20Object%20Reference) (OtherBodyIndex :type Integer))
  (bind _as_bp_player (Variables|Default|GetAs%20BP%20Player))
  (if (== OtherActor _as_bp_player)
    (Widget|SetVisibility (Variables|/Game/Game/WBP_ATH.WBP_ATH_C|GetImagEE (Variables|/Game/Game/BP_Player.BP_Player_C|GetATHref _as_bp_player)) "Hidden")))

(event OnComponentBeginOverlap(Box)
  (params (OverlappedComponent :type Primitive%20Component%20Object%20Reference) (OtherActor :type Actor%20Object%20Reference) (OtherComp :type Primitive%20Component%20Object%20Reference) (OtherBodyIndex :type Integer) (bFromSweep :type Boolean) (SweepResult :type Hit%20Result%20Structure%20%28by%20ref%29))
  (bind _as_bp_player (Variables|Default|GetAs%20BP%20Player))
  (Utilities|FlowControl|Sequence
    (:then_0
      (Utilities|Casting|CastToBP_Walls OtherActor)
      (Utilities|FlowControl|Delay 0.2)
      (Physics|SetSimulatePhysics (Variables|Default|GetCube) false)
      (Components|Activation|Deactivate (Variables|Default|GetAudio))
      (Variables|Default|SetcanKillEnemy false))
    (:then_1
      (if (== OtherActor _as_bp_player)
        (if (Variables|Default|GetcanBePropulse)
          (Widget|SetVisibility (Variables|/Game/Game/WBP_ATH.WBP_ATH_C|GetImagEE (Variables|/Game/Game/BP_Player.BP_Player_C|GetATHref _as_bp_player)) "Visible"))))))

(event OnComponentBeginOverlap(KillBox)
  (params (OverlappedComponent :type Primitive%20Component%20Object%20Reference) (OtherActor :type Actor%20Object%20Reference) (OtherComp :type Primitive%20Component%20Object%20Reference) (OtherBodyIndex :type Integer) (bFromSweep :type Boolean) (SweepResult :type Hit%20Result%20Structure%20%28by%20ref%29))
  (bind _asbp_enemy (Utilities|Casting|CastToBP_Enemy OtherActor))
  (if (Variables|Default|GetcanKillEnemy)
    (Actor|DestroyActor _asbp_enemy)))

(event Custom|PropulseBlock
  (bind _cube (Variables|Default|GetCube))
  ;[1 1 1] Donner une implusion au block
  (if (Variables|Default|GetcanBePropulse)
    (Physics|SetSimulatePhysics (Variables|Default|GetCube) true)
    (bind _output_get (Variables|Default|SetVectorPulse (Utilities|GetVectorPulse)))
    (if (or (> (.x _output_get) 1e+03) (< (.x _output_get) -1e+03))
      (Physics|AddImpulse _cube (Math|Vector|MakeVector (.x (Variables|Default|GetVectorPulse)) 0.0 0.0) "None" true)
      (Variables|Default|SetcanKillEnemy true :!label _label)
      (Components|Activation|Activate (Variables|Default|GetAudio) false)
      (elif (or (> (.y _output_get) 1e+03) (< (.y _output_get) -1e+03))
        (Physics|AddImpulse _cube (Math|Vector|MakeVector 0.0 (.y (Variables|Default|GetVectorPulse)) 0.0) "None" true)
        (goto _label)))))

(event Custom|MakeCubeOnSwitch
  (Variables|Default|SetcanBePropulse false)
  (Physics|SetSimulatePhysics (Variables|Default|GetCube) false))

(event EventBeginPlay
  (Variables|Default|SetLocInit (Transformation|GetWorldLocation (Variables|Default|GetDefaultSceneRoot)))
  (bind _asbp_player (Utilities|Casting|CastToBP_Player (Game|GetPlayerCharacter 0)))
  (Variables|Default|SetAs%20BP%20Player _asbp_player))

(fn ConstructionScript)