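; BP_Enemy is an enemy Blueprint that starts pursuit when its PawnSensing component sees a pawn.
; The sighting sets IsSeeingPlayer, which is never cleared here, and calls FollowPlayer, which issues AIMoveTo targeting the player controller rather than the character.
; An unconnected chain targets BP_Player with debug prints and a delayed retry on failure, but never runs.
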(event OnSeePawn(PawnSensing)
  (params (Pawn :type Pawn%20Object%20Reference))
  (Variables|Default|SetIsSeeingPlayer true)
  (CallFunction|FollowPlayer))

(event Custom|FollowPlayer
  (if (Variables|Default|GetIsSeeingPlayer)
    (AI|AIMoveTo self "0, 0, 0" (Game|GetPlayerController 0) 5.0 false)))

(event EventBeginPlay)

(fn ConstructionScript)